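; BP_STUProjectile is a weapon projectile Blueprint that handles cleanup of its effects and components on impact.
; OnHit runs a sequence of validity-checked steps that pause and hide the trace effect, destroy the point light and sphere, and stop the audio.
; The smoke trail has its spawn rate zeroed instead of being destroyed, so no new particles spawn.
; Movement and damage are absent from these graphs.
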(event `self.OnHit`
  (bind _tracefx (`self.TraceFX`))
  (bind _sphere (`self.Sphere`))
  (bind _pointlight (`self.PointLight`))
  (bind _tracesmokefx (`self.TraceSmokeFX`))
  (bind _audio (`self.Audio`))
  (`|ExecutionSequence`
    (:`then_0`
      (`/Engine/EditorBlueprintResources/StandardMacros.IsValid` _tracefx
        (:`Is Valid`
          (`NiagaraComponent.SetPaused` _tracefx true)
          (`SceneComponent.SetVisibility` _tracefx false true))))
    (:`then_1`
      (`/Engine/EditorBlueprintResources/StandardMacros.IsValid` _pointlight
        (:`Is Valid`
          (`ActorComponent.K2_DestroyComponent` _pointlight))))
    (:`then_2`
      (`/Engine/EditorBlueprintResources/StandardMacros.IsValid` _sphere
        (:`Is Valid`
          (`ActorComponent.K2_DestroyComponent` _sphere))))
    (:`then_3`
      (`/Engine/EditorBlueprintResources/StandardMacros.IsValid` _tracesmokefx
        (:`Is Valid`
          (`NiagaraComponent.SetVariableFloat` _tracesmokefx "SpawnRate" 0.0))))
    (:`then_4`
      (`/Engine/EditorBlueprintResources/StandardMacros.IsValid` _audio
        (:`Is Valid`
          (`AudioComponent.Stop` _audio))))))

(fn `UserConstructionScript`)